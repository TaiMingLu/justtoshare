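; BP_PanoramaCamera2 is a capture rig that steps along a straight line and saves a numbered PNG at each evenly spaced point.
; BeginPlay sets the hard-coded endpoints, image count and step size, then moves to the start.
; Tick works as a two-flag state machine: it captures from SceneCaptureComponentFront on arrival and advances only once the file exists on disk.
; Panorama console commands, a loop-based version and SaveCapturedImage logic are left unconnected.
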(event `self.ReceiveTick`
  (params (DeltaSeconds :type "Float (single-precision)"))
  (bind _returnvalue (`KismetStringLibrary.Concat_StrStr` "F:/outputs/" (`KismetStringLibrary.Conv_IntToString` (`self.CurrentPictureIndex`)) ".png"))
  (bind _returnvalue_2 (+ (`self.StartPoint`) (* (`self.MoveDistance`) (`self.CurrentPictureIndex`))))
  (`|ExecutionSequence`
    (:`then_0`
      (if (`self.atPosition`)
        _
        (elif (== (`self.K2_GetActorLocation`) _returnvalue_2)
          (set `self.atPosition` true)
          (`VictoryBPFunctionLibrary.CaptureComponent2D_SaveImage` (`self.SceneCaptureComponentFront`) _returnvalue))))
    (:`then_1`
      (if (not (`self.ImageSaved`))
        (bind _returnvalue_3 (`BlueprintFileUtilsBPLibrary.FileExists` _returnvalue))
        (if _returnvalue_3
          (set `self.ImageSaved` true)
          (set `self.CurrentPictureIndex` (+ (`self.CurrentPictureIndex`) 1))
          (if (< (`self.CurrentPictureIndex`) (`self.NumPictures `))
            (`KismetSystemLibrary.PrintString` (`KismetStringLibrary.Conv_IntToString` (`self.CurrentPictureIndex`)))
            (`self.K2_SetActorLocation` _returnvalue_2 :!label _label)
            (`|ExecutionSequence`
              (:`then_0`
                (set `self.atPosition` false))
              (:`then_1`
                (set `self.ImageSaved` false)))))))))

(event `self.ReceiveBeginPlay`
  (`KismetSystemLibrary.Delay` 0.0)
  (`|ExecutionSequence`
    (:`then_0`
      (set `self.NumPictures ` 50))
    (:`then_1`
      (set `self.CurrentPictureIndex` 0))
    (:`then_2`
      (set `self.StartPoint` (29180.0 -9270.0 430.0)))
    (:`then_3`
      (set `self.EndPoint` (28490.0 -9270.0 430.0)))
    (:`then_4`
      (set `self.MoveDistance` (/ (- (`self.EndPoint`) (`self.StartPoint`)) (- (`self.NumPictures `) 1))))
    (:`then_5`
      (goto _label))))

(fn `SaveCapturedImage`)

(fn `UserConstructionScript`)