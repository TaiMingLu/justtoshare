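; Panorama capture actor that steps a scene capture along a straight line and saves a numbered PNG at each stop.
; BeginPlay divides a hardcoded start-to-end path into evenly spaced positions, then teleports or saves nothing on Tick, doing all work in one loop.
; Each step busy-waits until the location matches and the image file exists in a fixed output folder.
; An earlier index-driven version and SaveCapturedImage experiments remain unconnected.
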(event `self.ReceiveBeginPlay`
  (bind _returnvalue (`self.K2_GetActorLocation`))
  (`KismetSystemLibrary.Delay` 0.0)
  (`|ExecutionSequence`
    (:`then_0`
      (set `self.NumPictures ` 50))
    (:`then_1`
      (set `self.CurrentPictureIndex` 0))
    (:`then_2`
      (set `self.StartPoint` (30000.0 -9270.0 430.0)))
    (:`then_3`
      (set `self.EndPoint` (21490.0 -9270.0 430.0)))
    (:`then_4`
      (set `self.MoveDistance` (/ (- (`self.EndPoint`) (`self.StartPoint`)) (- (`self.NumPictures `) 1))))
    (:`then_5`
      (for _index (range (`self.NumPictures `))
        (bind _returnvalue_2 (+ (`self.StartPoint`) (* (`self.MoveDistance`) _index)))
        (`self.K2_SetActorLocation` _returnvalue_2)
        (set `self.atPosition` false)
        (while (not (`self.atPosition`))
          (if (== _returnvalue _returnvalue_2)
            (set `self.atPosition` true)
            (`KismetSystemLibrary.PrintString` (`KismetStringLibrary.Conv_VectorToString` _returnvalue))))
        (bind _returnvalue_3 (`KismetStringLibrary.Concat_StrStr` "F:/outputs/" (`KismetStringLibrary.Conv_IntToString` _index) ".png"))
        (`VictoryBPFunctionLibrary.CaptureComponent2D_SaveImage` (`self.SceneCaptureComponent`) _returnvalue_3)
        (set `self.ImageSaved` false)
        (while (not (`self.ImageSaved`))
          (bind _returnvalue_4 (`BlueprintFileUtilsBPLibrary.FileExists` _returnvalue_3))
          (if _returnvalue_4
            (set `self.ImageSaved` true)
            (`KismetSystemLibrary.PrintString` (`KismetStringLibrary.Conv_IntToString` _index))))))))

(event `self.ReceiveTick`
  (params (DeltaSeconds :type "Float (single-precision)")))

(fn `SaveCapturedImage`)

(fn `UserConstructionScript`)