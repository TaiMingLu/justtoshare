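; Automated capture actor that saves six-direction panorama image sequences along random straight paths through the level.
; FindValidPath samples a start point and yaw within bounds, moving the player pawn there and flushing level streaming, until a line trace finds a clear path.
; Tick steps the actor along it, saving six scene captures as PNGs per position and polling for all files before advancing.
; Finished paths trigger new numbered iterations, with ray-traced captures enabled at BeginPlay.
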(event `self.ReceiveTick`
  (params (DeltaSeconds :type "Float (single-precision)"))
  (bind _iterationcount (`self.IterationCount`))
  (bind _returnvalue (`KismetStringLibrary.Concat_StrStr` (`self.IterationPath`) (`KismetStringLibrary.Conv_IntToString` (`self.CurrentPictureIndex`))))
  (bind _returnvalue_2 (+ (`self.StartPoint`) (* (`self.StepSize`) (`self.CurrentPictureIndex`))))
  (`|ExecutionSequence`
    (:`then_0`
      (if (`self.atPosition`)
        _
        (elif (== (`self.K2_GetActorLocation`) _returnvalue_2)
          (set `self.atPosition` true)
          (`|ExecutionSequence`
            (:`then_0`
              (bind _output_get (set `self.FrontSavePath` (`KismetStringLibrary.Concat_StrStr` _returnvalue "_front" ".png")))
              (`VictoryBPFunctionLibrary.CaptureComponent2D_SaveImage` (`self.SceneCaptureComponentFront`) _output_get))
            (:`then_1`
              (bind _output_get_2 (set `self.LeftSavePath` (`KismetStringLibrary.Concat_StrStr` _returnvalue "_left" ".png")))
              (`VictoryBPFunctionLibrary.CaptureComponent2D_SaveImage` (`self.SceneCaptureComponentLeft`) _output_get_2))
            (:`then_2`
              (bind _output_get_3 (set `self.RightSavePath` (`KismetStringLibrary.Concat_StrStr` _returnvalue "_right" ".png")))
              (`VictoryBPFunctionLibrary.CaptureComponent2D_SaveImage` (`self.SceneCaptureComponentRight`) _output_get_3))
            (:`then_3`
              (bind _output_get_4 (set `self.BackSavePath` (`KismetStringLibrary.Concat_StrStr` _returnvalue "_back" ".png")))
              (`VictoryBPFunctionLibrary.CaptureComponent2D_SaveImage` (`self.SceneCaptureComponenBack`) _output_get_4 (struct :`A` 1.0)))
            (:`then_4`
              (bind _output_get_5 (set `self.TopSavePath` (`KismetStringLibrary.Concat_StrStr` _returnvalue "_top" ".png")))
              (`VictoryBPFunctionLibrary.CaptureComponent2D_SaveImage` (`self.SceneCaptureComponentTop`) _output_get_5))
            (:`then_5`
              (bind _output_get_6 (set `self.BottomSavePath` (`KismetStringLibrary.Concat_StrStr` _returnvalue "_bottom" ".png")))
              (`VictoryBPFunctionLibrary.CaptureComponent2D_SaveImage` (`self.SceneCaptureComponentBottom`) _output_get_6))))))
    (:`then_1`
      (if (not (`self.ImageSaved`))
        (bind _returnvalue_3 (`BlueprintFileUtilsBPLibrary.FileExists` (`self.FrontSavePath`)))
        (bind _returnvalue_4 (`BlueprintFileUtilsBPLibrary.FileExists` (`self.LeftSavePath`)))
        (bind _returnvalue_5 (`BlueprintFileUtilsBPLibrary.FileExists` (`self.RightSavePath`)))
        (bind _returnvalue_6 (`BlueprintFileUtilsBPLibrary.FileExists` (`self.BackSavePath`)))
        (bind _returnvalue_7 (`BlueprintFileUtilsBPLibrary.FileExists` (`self.TopSavePath`)))
        (bind _returnvalue_8 (`BlueprintFileUtilsBPLibrary.FileExists` (`self.BottomSavePath`)))
        (if (and _returnvalue_3 _returnvalue_4 _returnvalue_5 _returnvalue_6 _returnvalue_7 _returnvalue_8)
          (set `self.ImageSaved` true)
          (set `self.CurrentPictureIndex` (+ (`self.CurrentPictureIndex`) 1))
          (if (< (`self.CurrentPictureIndex`) (`self.NumPictures `))
            (`KismetSystemLibrary.PrintString` (`KismetStringLibrary.Conv_IntToString` (`self.CurrentPictureIndex`)))
            (`self.K2_SetActorLocation` _returnvalue_2 :!label _label)
            (`KismetSystemLibrary.PrintString` (`KismetStringLibrary.Conv_VectorToString` _returnvalue_2))
            (`|ExecutionSequence`
              (:`then_0`
                (set `self.atPosition` false))
              (:`then_1`
                (set `self.ImageSaved` false)))
            (else
              (set `self.IterationCount` (+ (`self.IterationCount`) 1))
              (if (< _iterationcount 10000) :!label _label_2
                (`KismetSystemLibrary.PrintText` (`KismetTextLibrary.Conv_StringToText` (`KismetStringLibrary.Concat_StrStr` "In Iteration " (`KismetStringLibrary.Conv_IntToString` _iterationcount))))
                (`self.FindValidPath`)
                (`KismetSystemLibrary.PrintString` "Path Set")
                (bind _output_get_7 (set `self.IterationPath` (`KismetStringLibrary.Concat_StrStr` (`self.SavePath`) (`KismetStringLibrary.Conv_IntToString` (`self.IterationCount`)) "/")))
                (`KismetSystemLibrary.PrintString` "Starting the Iteration")
                (`|ExecutionSequence`
                  (:`then_0`
                    (`BlueprintFileUtilsBPLibrary.MakeDirectory` _output_get_7 true))
                  (:`then_1`
                    (`KismetSystemLibrary.PrintString` "Start Rendering")
                    (`|ExecutionSequence`
                      (:`then_0`
                        (set `self.NumPictures ` 50))
                      (:`then_1`
                        (set `self.CurrentPictureIndex` 0))
                      (:`then_2`
                        (`self.K2_SetActorRotation` (`KismetMathLibrary.Conv_VectorToRotator` (`self.StartRotation`))))
                      (:`then_3`
                        (set `self.StepSize` (/ (- (`self.EndPoint`) (`self.StartPoint`)) (- (`self.NumPictures `) 1))))
                      (:`then_4`
                        (`KismetSystemLibrary.PrintString` "Setting Camera Position")
                        (goto _label)))))))))))))

(event `self.ReceiveBeginPlay`
  (`KismetSystemLibrary.Delay` 5.0)
  (`KismetSystemLibrary.ExecuteConsoleCommand` "r.RayTracing.SceneCaptures 1" null)
  (set `self.IterationCount` 0)
  (goto _label_2))

(event `FindValidPath`
  (bind _returnvalue (`GameplayStatics.GetPlayerPawn` 0))
  (`self.SetActorHiddenInGame` (`GameplayStatics.GetPlayerPawn` 0) false)
  (`|ExecutionSequence`
    (:`then_0`
      (set `self.MoveDistance` 2000.0))
    (:`then_1`
      (set `self.PathIsValid` false))
    (:`then_2`
      (while (not (`self.PathIsValid`))
        (`KismetSystemLibrary.PrintString` "Sampling Path")
        (`|ExecutionSequence`
          (:`then_0`
            (bind _output_get (set `self.StartPoint` (`KismetMathLibrary.MakeVector` (`KismetMathLibrary.RandomFloatInRange` (`self.MinX`) (`self.MaxX`)) (`KismetMathLibrary.RandomFloatInRange` (`self.MinY`) (`self.MaxY`)) (`KismetMathLibrary.RandomFloatInRange` (`self.MinZ`) (`self.MaxZ`)))))
            (`KismetSystemLibrary.PrintString` (`KismetStringLibrary.Concat_StrStr` "Start Position: " (`KismetStringLibrary.Conv_VectorToString` _output_get))))
          (:`then_1`
            (bind _output_get_2 (set `self.StartRotation` (`KismetMathLibrary.Conv_RotatorToVector` (`KismetMathLibrary.MakeRotator` 0.0 0.0 (`KismetMathLibrary.RandomFloatInRange` -180.0 180.0)))))
            (`KismetSystemLibrary.PrintString` (`KismetStringLibrary.Concat_StrStr` "Rotation: " (`KismetStringLibrary.Conv_VectorToString` _output_get_2))))
          (:`then_2`
            (bind _output_get_3 (set `self.EndPoint` (+ (* (`KismetMathLibrary.GetForwardVector` (`KismetMathLibrary.Conv_VectorToRotator` (`self.StartRotation`))) (`self.MoveDistance`)) (`self.StartPoint`))))
            (`KismetSystemLibrary.PrintString` (`KismetStringLibrary.Concat_StrStr` "End Position: : " (`KismetStringLibrary.Conv_VectorToString` _output_get_3))))
          (:`then_3`
            (`self.K2_SetActorLocation` _returnvalue (`self.StartPoint`) false false)
            (`self.K2_SetActorRotation` _returnvalue (`KismetMathLibrary.Conv_VectorToRotator` (`self.StartRotation`)) false)
            (`GameplayStatics.FlushLevelStreaming`)
            (`KismetSystemLibrary.PrintString` "Set Camera and Render Scene"))
          (:`then_4`
            (bind (_outhit _returnvalue_2) (`KismetSystemLibrary.LineTraceSingle` (`self.StartPoint`) (`self.EndPoint`) "TraceTypeQuery3"))
            (`KismetSystemLibrary.PrintString` (`KismetStringLibrary.Concat_StrStr` "Hit: " (`KismetStringLibrary.Conv_BoolToString` _returnvalue_2)))
            (if _returnvalue_2
              (`KismetSystemLibrary.PrintString` "Invalid Path, Retrying")
              (else
                (set `self.PathIsValid` true))))))
      (`KismetSystemLibrary.PrintString` "Valid Path Sampled"))))

(fn `SaveCapturedImage`)

(fn `UserConstructionScript`)